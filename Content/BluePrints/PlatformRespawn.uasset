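; PlatformRespawn is a platform actor that falls after the player steps into its trigger, then respawns.
; The first player overlap destroys the trigger component and starts a delay timer, after which the platform mesh simulates physics.
; A second timer then spawns a fresh PlatformRespawn at the actor's transform with a particle effect and destroys the old actor, so the replacement starts with clean state.
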(event OnComponentBeginOverlap(PlatformFalls_Trigger)
  (params (OverlappedComponent :type Primitive%20Component%20Object%20Reference) (OtherActor :type Actor%20Object%20Reference) (OtherComp :type Primitive%20Component%20Object%20Reference) (OtherBodyIndex :type Integer) (bFromSweep :type Boolean) (SweepResult :type Hit%20Result%20Structure%20%28by%20ref%29))
  (if (== OtherActor (Game|GetPlayerCharacter 0))
    (Utilities|FlowControl|DoOnce false
      (:Completed
        (Utilities|FlowControl|Sequence
          (:then_0
            (bind _platformfalls_trigger (Variables|Default|GetPlatformFalls_Trigger)
              (:then
                (Components|DestroyComponent _platformfalls_trigger))
              (:else)))
          (:then_1
            (bind _returnvalue (Utilities|Time|SetTimerbyEvent (delegate Custom|Platform%20Falls) (Variables|Platform|GetPlatform%20Falls%20After)))))))))

(event Custom|Platform%20Falls
  (Utilities|Time|ClearandInvalidateTimerbyHandle (stale OnComponentBeginOverlap(PlatformFalls_Trigger) _returnvalue))
  (Physics|SetSimulatePhysics (Variables|Default|GetPlatform_SM) true)
  (bind _returnvalue (Utilities|Time|SetTimerbyEvent (delegate Custom|Respawn%20Platform) (Variables|Default|GetRespawn%20Platform%20After))))

(event Custom|Respawn%20Platform
  (Utilities|Time|ClearandInvalidateTimerbyHandle (stale Custom|Platform%20Falls _returnvalue))
  (Game|SpawnActorfromClass "PlatformRespawn_C" (Transformation|GetActorTransform) "Undefined" "MultiplyWithRoot" 0 0)
  (Effects|SpawnEmitteratLocation 0 (Transformation|GetActorLocation))
  (Actor|DestroyActor))

(event EventBeginPlay)

(event Collision|EventActorBeginOverlap
  (params (OtherActor :type Actor%20Object%20Reference)))

(event EventTick
  (params (DeltaSeconds :type Float%20%28single-precision%29)))

(fn ConstructionScript)