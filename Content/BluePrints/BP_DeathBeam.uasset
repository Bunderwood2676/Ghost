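; BP_DeathBeam is a configurable beam hazard that damages whatever registers a hit on its Beam component.
; On BeginPlay, boolean flags enable independent behaviors: timeline-driven yaw rotation, X/Y scale pulsing, X-axis movement of the base, and visibility blinking.
; Scaling and blinking re-trigger FlipFlops through Delay loops, while movement's FlipFlop fires only once, so its reverse branch never runs.
; Blinking toggles only visibility, leaving collision untouched.
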(event OnComponentHit(Beam)
  (params (HitComponent :type Primitive%20Component%20Object%20Reference) (OtherActor :type Actor%20Object%20Reference) (OtherComp :type Primitive%20Component%20Object%20Reference) (NormalImpulse :type Vector :default "0, 0, 0") (Hit :type Hit%20Result%20Structure%20%28by%20ref%29))
  (Game|Damage|ApplyDamage OtherActor 1.0 0 0))

(event EventBeginPlay
  ;[0.15 0.15 0.15 0.5] Rotation top, Scaling Top Middle, Movement Bottom Middle, Blinking Bottom
  (Utilities|FlowControl|Sequence
    (:then_0
      (if (Variables|Default|GetDoRotation)
        (bind _rotation (Timeline|Beam%20Rotate Play)
          (:Update
            (Transformation|SetWorldRotation (Variables|Default|GetBase) (Math|Rotator|MakeRotator 0.0 0.0 _rotation) false false)))))
    (:then_1
      (if (Variables|Default|GetDoRandomScale)
        (Utilities|FlowControl|FlipFlop :!label _label
          (:A
            (bind _scaling (Timeline|Scale Play)
              (:Update
                (Transformation|SetWorldScale3D (Variables|Default|GetBeam) (Math|Vector|MakeVector (.x (Math|Interpolation|VInterpTo "0.0,0.0,0.0" (Math|Vector|MakeVector (.x (Math|Vector|MakeVector (Math|Float|Clamp(Float) 1.0 0.2 _scaling) (Math|Float|Clamp(Float) 1.0 0.2 _scaling) 1.0)) (.y (Math|Vector|MakeVector (Math|Float|Clamp(Float) 1.0 0.2 _scaling) (Math|Float|Clamp(Float) 1.0 0.2 _scaling) 1.0)) 1.0) 1.0 4.0)) (.y (Math|Interpolation|VInterpTo "0.0,0.0,0.0" (Math|Vector|MakeVector (.x (Math|Vector|MakeVector (Math|Float|Clamp(Float) 1.0 0.2 _scaling) (Math|Float|Clamp(Float) 1.0 0.2 _scaling) 1.0)) (.y (Math|Vector|MakeVector (Math|Float|Clamp(Float) 1.0 0.2 _scaling) (Math|Float|Clamp(Float) 1.0 0.2 _scaling) 1.0)) 1.0) 1.0 4.0)) 7.0))
                (Utilities|FlowControl|Delay 2.5)
                (goto _label))))
          (:B
            (Timeline|Scale Reverse)))))
    (:then_2
      (if (Variables|Default|GetBeamMoveForward)
        (Utilities|FlowControl|FlipFlop
          (:A
            (bind _movement (Timeline|BeamMove Play)
              (:Update
                (Transformation|SetRelativeLocation (Variables|Default|GetBase) (Math|Vector|MakeVector _movement 0.0 0.0) false false))))
          (:B
            (Timeline|BeamMove Reverse)))))
    (:then_3
      (if (Variables|Default|GetBlinkingBeam)
        (Utilities|FlowControl|FlipFlop :!label _label_2
          (:A
            (Rendering|SetVisibility (Variables|Default|GetBeam) false false))
          (:B
            (Rendering|SetVisibility (Variables|Default|GetBeam) true false)))
        (Utilities|FlowControl|Delay (Variables|Default|GetBeamBlinkTimer))
        (goto _label_2)))))

(fn ConstructionScript)