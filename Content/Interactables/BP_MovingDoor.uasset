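; BP_MovingDoor is a door that slides open and closed in response to a linked pressure plate.
; On BeginPlay it casts LinkedInteractable to the pressure plate Blueprint and binds to its plate state change event.
; Activation plays a Timeline that lerps the mesh's relative location from zero to OpenOffset, and deactivation reverses it.
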(event Custom|OnDoorTriggered
  (params (IsActivated :type Boolean))
  (if IsActivated
    (bind _alpha (Timeline|Timeline Play)
      (:Update
        (Transformation|SetRelativeLocation (Variables|Default|GetStaticMesh) (Math|Vector|Lerp(Vector) "0, 0, 0" (Variables|Default|GetOpenOffset) _alpha) false false)))
    (else
      (Timeline|Timeline Reverse))))

(event EventBeginPlay
  (bind _linkedinteractable (Variables|Default|GetLinkedInteractable))
  (Utilities|IsValid _linkedinteractable
    (:Is%20Valid
      (bind _asbp_pressure_plate (Utilities|Casting|CastToBP+PressurePlate _linkedinteractable))
      (EventDispatchers|BindEventtoOnPlateStateChanged _asbp_pressure_plate (delegate Custom|OnDoorTriggered)))))

(event Collision|EventActorBeginOverlap
  (params (OtherActor :type Actor%20Object%20Reference)))

(event EventTick
  (params (DeltaSeconds :type Float%20%28single-precision%29)))

(fn ConstructionScript)