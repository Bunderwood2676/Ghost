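; BP_InteractableBase is a base interactable that shows a press animation and signals a linked door.
; Its sphere registers it as CurrentInteractable on overlapping third-person or ghost characters, but end overlap clears it only for the third-person character.
; OnInteractStateChanged plays a timeline that lowers the mesh and forwards the active state to LinkedDoor on every timeline update.
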(event OnComponentBeginOverlap(Sphere)
  (params (OverlappedComponent :type Primitive%20Component%20Object%20Reference) (OtherActor :type Actor%20Object%20Reference) (OtherComp :type Primitive%20Component%20Object%20Reference) (OtherBodyIndex :type Integer) (bFromSweep :type Boolean) (SweepResult :type Hit%20Result%20Structure%20%28by%20ref%29))
  (bind _asbp_third_person_character (Utilities|Casting|CastToBP_ThirdPersonCharacter OtherActor)
    (:then
      (Variables|/Game/ThirdPerson/Blueprints/BP_ThirdPersonCharacter.BP_ThirdPersonCharacter_C|SetCurrent%20Interactable _asbp_third_person_character self))
    (:CastFailed
      (bind _asbp_ghost_character (Utilities|Casting|CastToBP_GhostCharacter OtherActor))
      (Variables|/Game/ThirdPerson/Blueprints/BP_ThirdPersonCharacter.BP_ThirdPersonCharacter_C|SetCurrent%20Interactable _asbp_ghost_character self))))

(event OnComponentEndOverlap(Sphere)
  (params (OverlappedComponent :type Primitive%20Component%20Object%20Reference) (OtherActor :type Actor%20Object%20Reference) (OtherComp :type Primitive%20Component%20Object%20Reference) (OtherBodyIndex :type Integer))
  (bind _asbp_third_person_character (Utilities|Casting|CastToBP_ThirdPersonCharacter OtherActor))
  (if (== (Variables|/Game/ThirdPerson/Blueprints/BP_ThirdPersonCharacter.BP_ThirdPersonCharacter_C|GetCurrent%20Interactable _asbp_third_person_character) self)
    (Variables|/Game/ThirdPerson/Blueprints/BP_ThirdPersonCharacter.BP_ThirdPersonCharacter_C|SetCurrent%20Interactable _asbp_third_person_character 0)))

(event EventBeginPlay)

(event Collision|EventActorBeginOverlap
  (params (OtherActor :type Actor%20Object%20Reference)))

(event EventTick
  (params (DeltaSeconds :type Float%20%28single-precision%29)))

(event EventOnInteractStateChanged
  (params (Is%20Active :type Boolean))
  (bind _progress (Timeline|Anim_Press Play)
    (:Update
      (Transformation|SetRelativeLocation (Variables|Default|GetStaticMesh1) (Math|Vector|Lerp(Vector) "0, 0, 0" "0.000000,0.000000,-10.000000" _progress) false false)
      (Class|BPIInteractable|OnInteractStateChanged(Message) (Variables|Default|GetLinkedDoor) Is%20Active))))

(fn ConstructionScript)